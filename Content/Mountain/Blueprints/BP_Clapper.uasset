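; BP_Clapper is an actor, by its naming a bell clapper, that swings by rotating around its roll axis.
; BeginPlay stores the starting rotation and a second one offset in roll by a negative angle.
; Tick calls Play on the Swing timeline every frame, and its track lerps the actor's rotation between those two poses.
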(event EventBeginPlay
  (bind _returnvalue (Transformation|GetActorRotation))
  (bind (_roll _pitch _yaw) (Math|Rotator|BreakRotator _returnvalue))
  (Variables|Default|SetBellRight _returnvalue)
  (Variables|Default|SetBellLeft (Math|Rotator|MakeRotator (+ _roll -55.0) _pitch _yaw)))

(event EventTick
  (params (DeltaSeconds :type Float%20%28single-precision%29))
  (bind _swingtrack (Timeline|Swing Play)
    (:Update
      (Transformation|SetActorRotation (Math|Rotator|Lerp(Rotator) (Variables|Default|GetBellRight) (Variables|Default|GetBellLeft) _swingtrack)))))

(fn ConstructionScript)